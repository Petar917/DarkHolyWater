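; BP_Door is an interactable door actor that swings open and closed by 90 degrees.
; When a BP_ThirdPersonCharacter overlaps it, the door sets itself as that character's DoorOverlapping reference and tracks a PlayerIsOverlapping flag.
; Its InteractDoor event uses a FlipFlop to instantly add alternating yaw rotations to the Sphere component, with no interpolation.
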(event Custom|InteractDoor
  (bind _sphere (Variables|Default|GetSphere))
  (Utilities|FlowControl|FlipFlop
    (:A
      (Transformation|AddRelativeRotation _sphere "0.000000,-90.000000,0.000000" false false))
    (:B
      (Transformation|AddRelativeRotation _sphere "0.000000,90.000000,0.000000" false false))))

(event Collision|EventActorBeginOverlap
  (params (OtherActor :type Actor%20Object%20Reference))
  (bind _asbp_third_person_character (Utilities|Casting|CastToBP_ThirdPersonCharacter OtherActor))
  (Variables|/Game/ThirdPerson/Blueprints/BP_ThirdPersonCharacter.BP_ThirdPersonCharacter_C|SetDoorOverlapping _asbp_third_person_character self)
  (Variables|Default|SetbPlayerIsOverlapping true))

(event EventTick
  (params (DeltaSeconds :type Float%20%28single-precision%29)))

(event Collision|EventActorEndOverlap
  (params (OtherActor :type Actor%20Object%20Reference))
  (Utilities|Casting|CastToBP_ThirdPersonCharacter OtherActor)
  (Variables|Default|SetbPlayerIsOverlapping false))

(fn ConstructionScript)