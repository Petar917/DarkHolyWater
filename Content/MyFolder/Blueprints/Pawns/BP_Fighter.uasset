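; BP_Fighter is a fighter that deals a one-off hit to an assigned target fighter when play begins.
; On BeginPlay it applies its Damage to TargetFighter through Unreal's damage system, passing itself as the causer.
; Its AnyDamage handler subtracts incoming damage from Health, then, if the causer is another BP_Fighter, prints the attacker, victim, damage and remaining HP on screen.
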(event EventBeginPlay
  (Game|Damage|ApplyDamage (Variables|References|GetTargetFighter) (Variables|Stats|GetDamage) 0 self))

(event Collision|EventActorBeginOverlap
  (params (OtherActor :type Actor%20Object%20Reference)))

(event EventTick
  (params (DeltaSeconds :type Float%20%28single-precision%29)))

(event Game|Damage|EventAnyDamage
  (params (Damage :type Float%20%28single-precision%29) (DamageType :type Damage%20Type%20Object%20Reference) (InstigatedBy :type Controller%20Object%20Reference) (DamageCauser :type Actor%20Object%20Reference))
  (bind _output_get (Variables|Stats|SetHealth (- (Variables|Stats|GetHealth) Damage)))
  (bind _asbp_fighter (Utilities|Casting|CastToBP_Fighter DamageCauser))
  (Development|PrintString (Utilities|String|ToString(Text) (Utilities|Text|FormatText "{0} Attacks {1}  with {2} damage. {1} now has {3} HP." (Utilities|GetDisplayName _asbp_fighter) (Utilities|GetDisplayName self) Damage (Utilities|String|ToString(Float) _output_get))) true true "(R=1.000000,G=0.623814,B=0.356860,A=1.000000)" 2e+01))

(fn ConstructionScript)