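; Game mode that populates the level with BP_Fighter actors and defines a random free-for-all round of damage between them.
; On BeginPlay it draws BP_SpawnPoint actors at random without repeats, spawning a fighter at each until its loop limit or the points run out.
; StartBattle makes each stored fighter damage a random other fighter, re-rolling self-targets.
; Nothing connected in this graph calls StartBattle.
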(event Custom|StartBattle
  (bind _figthers (Variables|Default|GetFigthers))
  (for _array_element _figthers
    (Variables|Default|SetTargetRandom (.OutItem (Utilities|Array|Random _figthers)))
    (while (== (Variables|Default|GetTargetRandom) _array_element)
      ;[1 1 1] Reset Random Target
      (Variables|Default|SetTargetRandom (.OutItem (Utilities|Array|Random (Variables|Default|GetFigthers)))))
    ;[1 1 1] Apply Damage
    (Game|Damage|ApplyDamage (Variables|Default|GetTargetRandom) (Variables|/Game/MyFolder/Blueprints/Pawns/BP_Fighter.BP_Fighter_C|GetDamage _array_element) 0 _array_element)))

(event EventBeginPlay
  (CallFunction|SpawnFightersatSpawnPoints))

(event EventTick
  (params (DeltaSeconds :type Float%20%28single-precision%29)))

(fn ConstructionScript)

(fn SpawnFighter
  (params (Health :type Float%20%28double-precision%29) (Damage :type Float%20%28double-precision%29) (SpawnTransform :type Transform))
  (bind _returnvalue (Game|SpawnActorfromClass "/Game/MyFolder/Blueprints/Pawns/BP_Fighter.BP_Fighter_C" SpawnTransform "Undefined" "MultiplyWithRoot" 0 Health Damage 0))
  (return _returnvalue))

(fn SpawnFightersatSpawnPoints
  (bind _outactors (Actor|GetAllActorsOfClass "/Game/MyFolder/Blueprints/Misc/BP_SpawnPoint.BP_SpawnPoint_C"))
  (LocalVariables|SetSpawnPoints _outactors)
  (Utilities|FlowControl|ForLoopwithBreak 0 20
    (:LoopBody
      (if (Utilities|Array|IsNotEmpty (LocalVariables|GetSpawnPoints))
        (bind _output_get (LocalVariables|SetSpawnPointRandom (.OutItem (Utilities|Array|Random (LocalVariables|GetSpawnPoints)))))
        (Utilities|Array|RemoveItem (LocalVariables|GetSpawnPoints) _output_get)
        (bind _fighterspawned (CallFunction|SpawnFighter 1e+02 1e+01 (Transformation|GetActorTransform _output_get)))
        (Utilities|Array|Add (Variables|Default|GetFigthers) _fighterspawned)
        (else
          (Development|PrintString "error my ass" true true "(R=1.000000,G=0.000000,B=0.845590,A=1.000000)")
          (return))))))